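; Test actor that repeatedly spawns BP_FixedSeekProjectile instances and keeps them homing on a Target actor.
; A looping timer started on BeginPlay spawns a projectile at the actor's transform, passes it lifetime, delete delay and target location, and tracks it in an array.
; Every Tick prunes invalid projectiles from that array and rewrites each survivor's TargetLocation to the Target's current position.
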(event EventBeginPlay
  (Utilities|Time|SetTimerbyFunctionName 0 "FireProjectile" (Variables|Default|GettimeBetweenProjectiles) true))

(event Collision|EventActorBeginOverlap
  (params (OtherActor :type Actor%20Object%20Reference)))

(event EventTick
  (params (DeltaSeconds :type Float%20%28single-precision%29))
  (CallFunction|GuideProjectiles))

(fn ConstructionScript)

(fn FireProjectile
  (bind _returnvalue (Game|SpawnActorfromClass "/Game/TEST_Projectile/BP_FixedSeekProjectile.BP_FixedSeekProjectile_C" (Transformation|GetActorTransform) "Undefined" 0 0))
  (Variables|/Script/KOA_PROTO.BASE_Projectile|SetProjLifeTime _returnvalue (Variables|Default|Getlifetime))
  (Variables|/Script/KOA_PROTO.BASE_Projectile|SetTargetLocation _returnvalue (Transformation|GetActorLocation (Variables|Default|GetTarget)))
  (Variables|/Script/KOA_PROTO.BASE_Projectile|SetProjTimeBeforeDelete _returnvalue (Variables|Default|GettimeBeforeDelete))
  (Utilities|Array|Add (Variables|Default|GetcurrentProjectiles) _returnvalue))

(fn GuideProjectiles
  ;[1 1 1] Trim Current Projectiles array of non-existant projectiles
  (for _array_element (Variables|Default|GetcurrentProjectiles)
    (Utilities|IsValid _array_element
      (:Is%20Valid
        (Utilities|Array|Add (LocalVariables|GetnewArray) _array_element))))
  (Variables|Default|SetcurrentProjectiles (LocalVariables|GetnewArray))
  ;[1 1 1] Guide projectiles towards target
  (for _array_element_2 (Variables|Default|GetcurrentProjectiles)
    (Variables|/Script/KOA_PROTO.BASE_Projectile|SetTargetLocation _array_element_2 (Transformation|GetActorLocation (Variables|Default|GetTarget)))))