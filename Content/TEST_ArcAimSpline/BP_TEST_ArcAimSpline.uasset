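; Test actor for the ArcAimIndicator, which aims an arced shot from the player character toward the cursor.
; Every Tick feeds the indicator the character's location, gravity and minimum velocity, retargets it to the cursor and adds the character to its collision ignore list.
; Pressing E spawns a BP_TestBounceProjectile at the character, passing the indicator's computed start velocity and the same gravity.
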(event `self.ReceiveBeginPlay`
  (`self.EnableInput` (`GameplayStatics.GetPlayerController` 0)))

(event `self.ReceiveTick`
  (params (DeltaSeconds :type "Float (single-precision)"))
  (bind _arcaimindicator (`self.ArcAimIndicator`))
  (set `/Game/Jester/ArcAimIndicator/BP_ArcAimIndicator.StartPosition` (`self.K2_GetActorLocation` (`GameplayStatics.GetPlayerCharacter` 0)) _arcaimindicator)
  (set `/Game/Jester/ArcAimIndicator/BP_ArcAimIndicator.Gravity` (`self.Gravity`) _arcaimindicator)
  (`/Game/Jester/ArcAimIndicator/BP_ArcAimIndicator.SetTargetToCursor` (`self.ArcAimIndicator`))
  (`KismetArrayLibrary.Array_Add` (`/Game/Jester/ArcAimIndicator/BP_ArcAimIndicator.IgnoredActorsForCollision` (`self.ArcAimIndicator`)) (`GameplayStatics.GetPlayerCharacter` 0))
  (set `/Game/Jester/ArcAimIndicator/BP_ArcAimIndicator.MinInitialVelocity` (`self.MinVelocity`) (`self.ArcAimIndicator`)))

(event `Key|E`
  (params (Key :type "Key Structure" :default "AnyKey"))
  (:`Pressed`
    (`|SpawnActorFromClass` "/Game/TEST/BP_TestBounceProjectile.BP_TestBounceProjectile_C" (`KismetMathLibrary.MakeTransform` (`self.K2_GetActorLocation` (`GameplayStatics.GetPlayerCharacter` 0))) "Undefined" "OverrideRootScale" null (`/Game/Jester/ArcAimIndicator/BP_ArcAimIndicator.GetTargetStartVelocity` (`self.ArcAimIndicator`)) (`self.Gravity`))))

(fn `UserConstructionScript`)