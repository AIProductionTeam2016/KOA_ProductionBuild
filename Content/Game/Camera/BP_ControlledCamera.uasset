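; Side-view camera actor that follows the Jester player through switchable modes; Average Zoom is an empty stub.
; Tick runs the current mode and moves the actor, blending from the previous position after mode changes.
; Player Track holds fixed depth, while a looping timer computes accelerated/decelerated vertical velocity toward the player.
; Screen-edge bounds set a horizontal scroll direction that is never applied to movement, and debug lines show the zones.
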(event Custom|CustomTick
  (Utilities|Time|SetTimerbyEvent (delegate Custom|Milliseconds) (Variables|Default|GetcustomTickTime) true))

(event Custom|Milliseconds
  (CallFunction|CustomTickCameraMode))

(event EventBeginPlay
  ;[1 1 1] Get player reference
  (bind _aspcbp_jester (Utilities|Casting|CastToPCBP_Jester (Game|GetPlayerCharacter 0)))
  (Variables|Default|Setref_Player _aspcbp_jester)
  (CallFunction|StartCurrentCameraMode)
  (CallFunction|CustomTick))

(event Collision|EventActorBeginOverlap
  (params (OtherActor :type Actor%20Object%20Reference)))

(event EventTick
  (params (DeltaSeconds :type Float%20%28single-precision%29))
  (CallFunction|DoCurrentCameraMode DeltaSeconds)
  ;[1 1 1] Start transition if we changed modes
  (if (Utilities|Enum|NotEqual(Enum) (Variables|Default|GetcameraMode) (Variables|Default|GetcameraModeEdgeDetect))
    (CallFunction|StartTransition)
    (CallFunction|StartCurrentCameraMode))
  (Variables|Default|SetcameraModeEdgeDetect (Variables|Default|GetcameraMode))
  (CallFunction|DoTransition DeltaSeconds))

(fn ConstructionScript)

(fn DoTransition
  (params (deltaSeconds :type Float%20%28single-precision%29))
  (Variables|Default|Settransition_Timer (Math|Float|Max(Float) 0.0 (- (Variables|Default|Gettransition_Timer) deltaSeconds)))
  (Transformation|SetActorLocation (Math|Vector|Lerp(Vector) (Variables|Default|GetTargetPos) (Variables|Default|GetPreviousPos) (/ (Variables|Default|Gettransition_Timer) (Variables|Default|Gettransition_TotalSeconds))) false true))

(fn DoModePlayerTrack
  (params (deltaSeconds :type Float%20%28single-precision%29))
  (bind _returnvalue (Game|GetPlayerController 0))
  (bind _ref_player (Variables|Default|Getref_Player))
  (bind _returnvalue_2 (Transformation|GetActorLocation _ref_player))
  (bind _screenposition (Class|GameplayStatics|ProjectWorldtoScreen _returnvalue _returnvalue_2))
  (bind _x (Math|Vector2D|BreakVector2D _screenposition))
  (bind _newx (Utilities|DivbyScreenWidth _x))
  (bind _output_get (Variables|Default|SetTargetPos (+ (Variables|Default|GetTargetPos) (* (Variables|Default|GetVelocity) deltaSeconds))))
  (Variables|Default|SetTargetPos (Math|Vector|MakeVector (Variables|PlayerTrack|GetPT_Depth) (.Y (Math|Vector|BreakVector _output_get)) (.Z (Math|Vector|BreakVector _output_get))))
  (if (<= _newx (Variables|PlayerTrack|GetPT_BoundXPos))
    (Variables|PlayerTrack|SetPT_scrollLeft true)
    (Variables|PlayerTrack|SetPT_scrollRight false)
    (elif (>= _newx (- 1.0 (Variables|PlayerTrack|GetPT_BoundXPos)))
      (Variables|PlayerTrack|SetPT_scrollLeft false)
      (Variables|PlayerTrack|SetPT_scrollRight true)))
  (PlayerTrack|DrawDebugPlayerTrack))

(fn DoModeAverageZoom
  (params (deltaSeconds :type Float%20%28single-precision%29)))

(fn StartTransition
  (Variables|Default|SetPreviousPos (Variables|Default|GetTargetPos))
  (Variables|Default|Settransition_Timer (Variables|Default|Gettransition_TotalSeconds)))

(fn DoCurrentCameraMode
  (params (deltaSeconds :type Float%20%28single-precision%29))
  (switch Utilities|FlowControl|Switch|SwitchonECameraMode (Variables|Default|GetcameraMode)
    (:NewEnumerator0
      (PlayerTrack|DoModePlayerTrack deltaSeconds)
      (PlayerTrack|DrawDebugPlayerTrack))
    (:NewEnumerator1
      (AverageZoom|DoModeAverageZoom deltaSeconds))))

(fn StartModePlayerTrack
  (bind _ref_player (Variables|Default|Getref_Player))
  (bind _returnvalue (Transformation|GetActorLocation _ref_player))
  (bind (_x _y _z) (Math|Vector|BreakVector _returnvalue))
  (Variables|Default|SetTargetPos (Math|Vector|MakeVector (Variables|PlayerTrack|GetPT_Depth) _y _z))
  (Variables|PlayerTrack|SetPT_scrollLeft false)
  (Variables|PlayerTrack|SetPT_scrollRight false))

(fn StartCurrentCameraMode
  (switch Utilities|FlowControl|Switch|SwitchonECameraMode (Variables|Default|GetcameraMode)
    (:NewEnumerator0
      (PlayerTrack|StartModePlayerTrack))
    (:NewEnumerator1
      (AverageZoom|StartModeAverageZoom))))

(fn StartModeAverageZoom)

(fn DrawDebugPlayerTrack
  (bind _pt_targetxpos (Variables|PlayerTrack|GetPT_TargetXPos))
  (bind _pt_targetxpos_2 (Variables|PlayerTrack|GetPT_TargetXPos))
  (bind _pt_boundxpos (Variables|PlayerTrack|GetPT_BoundXPos))
  (bind _pt_boundxpos_2 (Variables|PlayerTrack|GetPT_BoundXPos))
  (bind _returnvalue (- 1.0 _pt_boundxpos_2))
  (bind _returnvalue_2 (- 1.0 _pt_targetxpos_2))
  (CallFunction|DrawScreenDebugLine (Math|Vector2D|MakeVector2D 0.2 0.5) (Math|Vector2D|MakeVector2D 0.8 0.5) "(R=0.558059,G=0.575000,B=0.562294,A=1.000000)")
  (CallFunction|DrawScreenDebugLine (Math|Vector2D|MakeVector2D _pt_targetxpos 0.2) (Math|Vector2D|MakeVector2D _pt_targetxpos 0.8) "(R=1.000000,G=0.000000,B=0.000000,A=1.000000)")
  (CallFunction|DrawScreenDebugLine (Math|Vector2D|MakeVector2D _returnvalue_2 0.2) (Math|Vector2D|MakeVector2D _returnvalue_2 0.8) "(R=1.000000,G=0.000000,B=0.000000,A=1.000000)")
  (CallFunction|DrawScreenDebugLine (Math|Vector2D|MakeVector2D _pt_boundxpos 0.2) (Math|Vector2D|MakeVector2D _pt_boundxpos 0.8) "(R=1.000000,G=0.477000,B=0.000000,A=1.000000)")
  (CallFunction|DrawScreenDebugLine (Math|Vector2D|MakeVector2D _returnvalue 0.2) (Math|Vector2D|MakeVector2D _returnvalue 0.8) "(R=1.000000,G=0.476841,B=0.000000,A=1.000000)"))

(fn DrawScreenDebugLine
  (params (Start :type Vector%202D%20Structure) (End :type Vector%202D%20Structure) (Color :type Linear%20Color%20Structure))
  (bind _returnvalue (Game|GetPlayerController 0))
  (bind (_x _y) (Math|Vector2D|BreakVector2D Start))
  (bind (_x_2 _y_2) (Math|Vector2D|BreakVector2D End))
  (bind _newx (Utilities|TimesScreenWidth _x))
  (bind _newy (Utilities|TimesScreenHeight _y))
  (bind _newx_2 (Utilities|TimesScreenWidth _x_2))
  (bind _newy_2 (Utilities|TimesScreenHeight _y_2))
  (bind _returnvalue_2 (Math|Vector2D|MakeVector2D _newx_2 _newy_2))
  (bind _returnvalue_3 (Math|Vector2D|MakeVector2D _newx _newy))
  (bind (_worldposition _worlddirection) (Class|GameplayStatics|DeprojectScreentoWorld _returnvalue _returnvalue_2))
  (bind (_worldposition_2 _worlddirection_2) (Class|GameplayStatics|DeprojectScreentoWorld _returnvalue _returnvalue_3))
  (Rendering|Debug|DrawDebugLine (+ _worldposition_2 (* _worlddirection_2 2e+02)) (+ _worldposition (* _worlddirection 2e+02)) Color 0.02 1.0))

(fn CustomTickCameraMode
  (switch Utilities|FlowControl|Switch|SwitchonECameraMode (Variables|Default|GetcameraMode)
    (:NewEnumerator0
      (PlayerTrack|CustomTickPlayerTrack))))

(fn CustomTickPlayerTrack
  (if (< (Math|Float|Absolute(Float) (.Z (Math|Vector|BreakVector (- (Transformation|GetActorLocation (Variables|Default|Getref_Player)) (Variables|Default|GetTargetPos))))) (LocalVariables|GetzTolerance))
    (Variables|Default|SetVelocity (* (Variables|Default|GetVelocity) "1.000000,1.000000, 0"))
    (else
      (Variables|Default|SetVelocity (Math|Vector|MakeVector (.X (Math|Vector|BreakVector (Variables|Default|GetVelocity))) (.Y (Math|Vector|BreakVector (Variables|Default|GetVelocity))) (CallFunction|PhysMoveOverTime (.Z (Math|Vector|BreakVector (Variables|Default|GetTargetPos))) (.Z (Math|Vector|BreakVector (Transformation|GetActorLocation (Variables|Default|Getref_Player)))) (.Z (Math|Vector|BreakVector (Variables|Default|GetVelocity))) 25.0 1e+01 (Variables|Default|GetcustomTickTime))))))
  (if (or (Variables|PlayerTrack|GetPT_scrollLeft) (Variables|PlayerTrack|GetPT_scrollRight))
    (LocalVariables|SetxScrollDir (- (Math|Conversions|ToInteger(Boolean) (Variables|PlayerTrack|GetPT_scrollLeft)) (Math|Conversions|ToInteger(Boolean) (Variables|PlayerTrack|GetPT_scrollRight))))))

(fn DoModePlayerTrackLERP
  (params (deltaSeconds :type Float%20%28single-precision%29))
  (bind _returnvalue (Transformation|GetActorLocation))
  (bind (_x _y _z) (Math|Vector|BreakVector _returnvalue))
  (Variables|Default|SetTargetPos (Math|Vector|MakeVector _x _y (Utilities|LerpOverTime _z (.Z (Math|Vector|BreakVector (Transformation|GetActorLocation (Variables|Default|Getref_Player)))) 0.9 deltaSeconds))))

(fn PhysMoveOverTime
  (params (Start :type Float%20%28single-precision%29) (End :type Float%20%28single-precision%29) (CurrentVelocity :type Float%20%28single-precision%29) (Acceleration :type Float%20%28single-precision%29) (Deceleration :type Float%20%28single-precision%29) (Delta%20Seconds :type Float%20%28single-precision%29))
  (LocalVariables|SetDelta Delta%20Seconds)
  (LocalVariables|SetVelTimesDelta (* CurrentVelocity Delta%20Seconds))
  (LocalVariables|SetAccTimesDelta (* Acceleration (LocalVariables|GetDelta)))
  (LocalVariables|SetDecTimesDelta (* Deceleration (LocalVariables|GetDelta)))
  (LocalVariables|SetOffset (- End Start))
  (return (/ (+ (LocalVariables|GetVelTimesDelta) (* (Math|Float|SelectFloat (LocalVariables|GetAccTimesDelta) (* (Math|Float|Min(Float) (Math|Float|Absolute(Float) (|((vel*vel)/(2*ofs)) (LocalVariables|GetVelTimesDelta) (LocalVariables|GetOffset))) (Math|Float|Absolute(Float) (LocalVariables|GetVelTimesDelta))) -1.0) (or (!= (Math|Float|Sign(Float) (LocalVariables|GetVelTimesDelta)) (Math|Float|Sign(Float) (LocalVariables|GetOffset))) (> (|(0-(((vel*vel)-((2*dec)*ofs))/(2*(acc+dec)))) (LocalVariables|GetVelTimesDelta) (LocalVariables|GetDecTimesDelta) (Math|Float|Absolute(Float) (LocalVariables|GetOffset)) (LocalVariables|GetAccTimesDelta)) 0.0))) (Math|Float|Sign(Float) (LocalVariables|GetOffset)))) (LocalVariables|GetDelta))))