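; Cat guard enemy NPC character that moves along the Y axis and exposes attack, flinch and health state.
; On BeginPlay it links itself to its health bar widget; once dead and grounded, it disables capsule collision.
; Otherwise each Tick sweeps the actor forward and teleports it back, flagging blocking surfaces too steep to land on as walls.
; Attacks snap yaw to face along ±Y, and flinching cancels the primary attack.
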(event EventBeginPlay
  ;[1 1 1] Set REF_EnemyHPBar
  (bind _aswbp_ui_enemy_health_bar (Utilities|Casting|CastToWBP_UI_EnemyHealthBar (UserInterface|GetUserWidgetObject (Variables|Default|GetEnemyHealthBar))))
  (Variables|/Game/UI/EnemyUI/WBP_UI_EnemyHealthBar.WBP_UI_EnemyHealthBar_C|SetREF_BASE_Enemy _aswbp_ui_enemy_health_bar self))

(event EventActorBeginOverlap
  (params (OtherActor :type Actor%20Object%20Reference)))

(event EventTick
  (params (DeltaSeconds :type Float%20%28single-precision%29))
  (if (and (Class|KOABASEEnemyCharacter|GetIsDead self) (not (AI|Components|NavMovement|IsFalling (Variables|Character|GetCharacterMovement))))
    (Collision|SetCollisionEnabled (Variables|Default|GetCapsuleComponent) "NoCollision")
    (else
      (CallFunction|TestforWall))))

(fn ConstructionScript)

(fn TestforWall
  (bind _output_get (LocalVariables|SetPrevLocation (Transformation|GetActorLocation)))
  (bind _sweephitresult (Transformation|SetActorLocation (+ _output_get (* (Transformation|GetActorForwardVector) (LocalVariables|GetSWEEP_OFFSET_AMOUNT))) true true))
  (bind _output_get_2 (Variables|Default|SethasWallInFront (and (.bBlockingHit (Collision|BreakHitResult _sweephitresult)) (> (Class|KismetMathLibrary|DegAcos (Math|Vector|DotProduct (.Normal (Collision|BreakHitResult _sweephitresult)) "0, 0,1.000000")) (Variables|Default|GetmaxAngleToLand)))))
  (Transformation|SetActorLocation (LocalVariables|GetPrevLocation) false true))

(fn GetHasWallinFront
  (return (Variables|Default|GethasWallInFront)))

(fn Attack
  (Variables|Default|SetisAttacking true)
  (CallFunction|RotatetoFaceY))

(fn EndAttacking
  (Variables|Default|SetisAttacking false))

(fn Flinch
  (Variables|Default|SetisFlinching true)
  (Variables|Default|SetisAttacking false))

(fn EndFlinching
  (Variables|Default|SetisFlinching false))

(fn GetHealth
  (return (Class|KOABASEEnemyCharacter|GetHPCurr)))

(fn GetIsFlinching
  (return (Variables|Default|GetisFlinching)))

(fn GetIsAttacking
  (return (or (Variables|Default|GetisAttacking) (Variables|Default|GetisAttacking2))))

(fn RotatetoFaceY
  (bind _returnvalue (Transformation|GetActorRotation))
  (bind (_roll _pitch) (Math|Rotator|BreakRotator _returnvalue))
  (bind (_roll_2 _pitch_2) (Math|Rotator|BreakRotator _returnvalue))
  (if (<= 0.0 (.Y (Math|Vector|BreakVector (Transformation|GetActorForwardVector))))
    (Transformation|SetActorRotation (Math|Rotator|MakeRotator _roll_2 _pitch_2 9e+01))
    (else
      (Transformation|SetActorRotation (Math|Rotator|MakeRotator _roll _pitch -9e+01)))))

(fn RotatetoFacePos
  (params (position :type Vector))
  (bind _returnvalue (Transformation|GetActorRotation))
  (bind (_roll _pitch) (Math|Rotator|BreakRotator _returnvalue))
  (bind (_roll_2 _pitch_2) (Math|Rotator|BreakRotator _returnvalue))
  (if (<= 0.0 (.Y (Math|Vector|BreakVector (- position (Transformation|GetActorLocation)))))
    (Transformation|SetActorRotation (Math|Rotator|MakeRotator _roll_2 _pitch_2 9e+01))
    (else
      (Transformation|SetActorRotation (Math|Rotator|MakeRotator _roll _pitch -9e+01)))))

(fn Attack2
  (Variables|Default|SetisAttacking2 true)
  (CallFunction|RotatetoFaceY))

(fn EndAttacking2
  (Variables|Default|SetisAttacking2 false))