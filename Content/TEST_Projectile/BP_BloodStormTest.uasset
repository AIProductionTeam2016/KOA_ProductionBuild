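; BP_BloodStormTest is a test projectile spawner that launches squiggly projectiles at a Target, followed by helix projectile bursts.
; A looping timer spawns each squiggly projectile, stores it and sets a timer for its lifetime.
; Tick prunes destroyed squiggly projectiles and updates the rest with the Target's current location.
; That timer spawns NumProjectiles helix projectiles at the Target's location, with their target-location assignment left disconnected.
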(event EventBeginPlay
  (Utilities|Time|SetTimerbyFunctionName 0 "FireSquigglyProjectile" (Variables|Default|GettimeBetweenSquiggly) true))

(event Collision|EventActorBeginOverlap
  (params (OtherActor :type Actor%20Object%20Reference)))

(event EventTick
  (params (DeltaSeconds :type Float%20%28single-precision%29))
  (CallFunction|GuideProjectiles))

(fn ConstructionScript)

(fn FireSquigglyProjectile
  (bind _returnvalue (Game|SpawnActorfromClass "/Game/TEST_Projectile/BP_SquigglyProjectile.BP_SquigglyProjectile_C" (Math|Transform|MakeTransform (Transformation|GetActorLocation)) "Undefined" 0 0))
  (Variables|/Script/KOA_PROTO.AMTA_Projectile_Squiggly|SetProjLifeTime _returnvalue (Variables|Default|GetlifetimeSquiggly))
  (Variables|/Script/KOA_PROTO.BASE_Projectile|SetTargetLocation _returnvalue (Transformation|GetActorLocation (Variables|Default|GetTarget)))
  (Variables|/Script/KOA_PROTO.AMTA_Projectile_Squiggly|SetProjTimeBeforeDelete _returnvalue (Variables|Default|GettimeBeforeDeleteSquiggly))
  (Utilities|Array|Add (Variables|Default|GetcurrentProjectilesSquiggly) _returnvalue)
  (Utilities|Time|SetTimerbyFunctionName 0 "FireMultHelixProjectiles" (Variables|Default|GetlifetimeSquiggly)))

(fn GuideProjectiles
  ;[1 1 1] Trim Current Projectiles array of non-existant projectiles
  (for _array_element (Variables|Default|GetcurrentProjectilesSquiggly)
    (Utilities|IsValid _array_element
      (:Is%20Valid
        (Utilities|Array|Add (LocalVariables|GetnewArray) _array_element))))
  (Variables|Default|SetcurrentProjectilesSquiggly (LocalVariables|GetnewArray))
  ;[1 1 1] Guide projectiles towards target
  (for _array_element_2 (Variables|Default|GetcurrentProjectilesSquiggly)
    (Variables|/Script/KOA_PROTO.BASE_Projectile|SetTargetLocation _array_element_2 (Transformation|GetActorLocation (Variables|Default|GetTarget)))))

(fn FireHelixProjectile
  (bind _returnvalue (Game|SpawnActorfromClass "/Game/TEST_Projectile/BP_HelixSeekProjectile.BP_HelixSeekProjectile_C" (Math|Transform|MakeTransform (Transformation|GetActorLocation (Variables|Default|GetTarget))) "Undefined" 0 0)))

(fn FireMultHelixProjectiles
  (for _index (range 1 (Variables|Default|GetnumProjectiles))
    (CallFunction|FireHelixProjectile)))