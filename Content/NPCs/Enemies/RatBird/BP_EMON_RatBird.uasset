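; RatBird enemy NPC Blueprint that runs simple custom physics for landing, sliding and falling.
; Each tick it probes for floor with a tiny swept downward move, then teleports back to its original location.
; A hit normal within the landing angle counts as floor and damps only Y velocity.
; Otherwise, gravity is added to the movement component's velocity every tick, without delta-time scaling.
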(event EventBeginPlay)

(event EventActorBeginOverlap
  (params (OtherActor :type Actor%20Object%20Reference)))

(event EventTick
  (params (DeltaSeconds :type Float%20%28single-precision%29))
  (CallFunction|TestforFloorandApplyFriction)
  (CallFunction|ApplyGravity))

(fn ConstructionScript)

(fn ApplyGravity
  (if (not (Variables|Default|GetisOnFloor))
    (Variables|/Script/Engine.MovementComponent|SetVelocity (Variables|Default|GetMovementComponent) (+ (Variables|/Script/Engine.MovementComponent|GetVelocity (Variables|Default|GetMovementComponent)) (Variables|Default|Getgravity)))))

(fn TestforFloorandApplyFriction
  (bind _output_get (LocalVariables|SetPrevLocation (Transformation|GetActorLocation)))
  (bind _sweephitresult (Transformation|SetActorLocation (- _output_get (LocalVariables|GetSMALL_Z_VECTOR)) true true))
  (bind _output_get_2 (Variables|Default|SetisOnFloor (<= (Class|KismetMathLibrary|DegAcos (Math|Vector|DotProduct (.Normal (Collision|BreakHitResult _sweephitresult)) "0, 0,1.000000")) (Variables|Default|GetminAngleToLand))))
  (Transformation|SetActorLocation (LocalVariables|GetPrevLocation) false true)
  (if _output_get_2
    (Variables|/Script/Engine.MovementComponent|SetVelocity (Variables|Default|GetMovementComponent) (Math|Vector|MakeVector (.X (Math|Vector|BreakVector (Variables|/Script/Engine.MovementComponent|GetVelocity (Variables|Default|GetMovementComponent)))) (* (.Y (Math|Vector|BreakVector (Variables|/Script/Engine.MovementComponent|GetVelocity (Variables|Default|GetMovementComponent)))) (Variables|Default|GetslidingFrictionMult)) (.Z (Math|Vector|BreakVector (Variables|/Script/Engine.MovementComponent|GetVelocity (Variables|Default|GetMovementComponent))))))))