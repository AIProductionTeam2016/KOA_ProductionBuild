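; AI controller for the Cat Guard enemy NPC that initializes its blackboard and starts its behavior tree.
; On BeginPlay it casts the controlled pawn to the Cat Guard character, stopping if that fails.
; It then seeds BB_CatGuardBlackboard with the pawn's patrol target count, first node index, patrolling state and starting location.
; It finally runs BT_CatGuardBehavior and has no Tick or other logic of its own.
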(event `self.ReceiveBeginPlay`
  (bind _asbp_enpc_00_cat_guard_character (cast `/Game/NPCs/Enemies/IMPORTED_REF_CGAI/BP_ENPC_00_CatGuardCharacter` (`self.K2_GetPawn`)))
  (bind _blackboardcomponent (`self.UseBlackboard` "/Game/NPCs/Enemies/CatGuard/AI/BB_CatGuardBlackboard.BB_CatGuardBlackboard"))
  (`BlackboardComponent.SetValueAsInt` _blackboardcomponent (`self.BBN_TotalNumPatrolNodes`) (`KismetArrayLibrary.Array_Length` (`/Game/NPCs/Enemies/IMPORTED_REF_CGAI/BP_ENPC_00_CatGuardCharacter.PatrolTargets` _asbp_enpc_00_cat_guard_character)))
  (`BlackboardComponent.SetValueAsInt` _blackboardcomponent (`self.BBN_CurrentPatrolNodeIndex`) 0)
  (`BlackboardComponent.SetValueAsEnum` _blackboardcomponent (`self.BBN_CurrentState`) (`self.EState_Patrolling`))
  (`BlackboardComponent.SetValueAsVector` _blackboardcomponent (`self.BBN_StartingPoint`) (`self.K2_GetActorLocation` (`self.K2_GetPawn`)))
  (`self.RunBehaviorTree` "/Game/NPCs/Enemies/CatGuard/AI/BT_CatGuardBehavior.BT_CatGuardBehavior"))

(event `self.ReceiveTick`
  (params (DeltaSeconds :type "Float (single-precision)")))

(fn `UserConstructionScript`)