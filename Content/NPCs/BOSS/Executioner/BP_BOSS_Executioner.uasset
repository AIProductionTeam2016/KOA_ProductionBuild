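; Executioner boss character that manages its health-bar UI, fight stage and the reward for its defeat.
; BeginPlay creates the boss HP widget and caches the Jester player; a start-fight event shows the widget.
; While alive, Tick sets the current stage by comparing HP ratio against a threshold array.
; Once dead, Tick repeatedly disables capsule collision, removes the UI and unlocks Blood Storm on the Jester's current artifact.
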(event Custom|EVENT_UnlockBloodStorm
  ;[1 1 1] EVENT: UNLOCK BLOOD STORM
  (Variables|/Script/KOA_PROTO.KOA_BASE_Artifact|SetIsArtifactStormUnlocked (Class|KOAPROTOCharacter|GetCurrArtifactReference (Variables|Jester|GetREF_Jester)) true))

(event Custom|EVENT_StartBossFight
  ;[1 1 1] EVENT: Start Boss Fight
  (UserInterface|Viewport|AddtoViewport (stale EventBeginPlay _output_get_2) 0))

(event EventTick
  (params (DeltaSeconds :type Float%20%28single-precision%29))
  ;[1 1 1] TICK
  (if (Class|KOABASEEnemyCharacter|GetIsDead (Variables|Self|GetREF_BOSS_Executioner))
    (Collision|SetCollisionEnabled (Variables|Default|GetCapsuleComponent) "NoCollision")
    (Widget|RemovefromParent (Variables|UI|GetREF_UI))
    (if (Class|KOABASEEnemyCharacter|GetIsDead self)
      (CallFunction|EVENTUnlockBloodStorm))
    (else
      ;[1 1 1] Set Stage
      (CallFunction|SetStage))))

(event EventBeginPlay
  ;[1 1 1] EVENT: Begin Play
  (bind _output_get (Variables|Self|SetREF_BOSS_Executioner self))
  (bind _returnvalue (UserInterface|CreateWidget "/Game/UI/NPC/WBP_UI_BOSS_HPBard.WBP_UI_BOSS_HPBard_C"))
  (bind _output_get_2 (Variables|UI|SetREF_UI _returnvalue))
  (Default|SetREFBOSS _output_get_2 _output_get)
  (bind _asbp_pc_jester (Utilities|Casting|CastToBP_PC_Jester (Game|GetPlayerCharacter 0)))
  (Variables|Jester|SetREF_Jester _asbp_pc_jester))

(fn ConstructionScript)

(fn SetStage
  (for (_array_element _array_index) (LocalVariables|GetStageThresholds)
    (if (<= (/ (Class|KOABASEEnemyCharacter|GetHPCurr) (Class|KOABASEEnemyCharacter|GetHPMax)) _array_element)
      (Variables|Default|SetcurrentStage (+ _array_index 1)))))

(fn GetStage
  (return (Variables|Default|GetcurrentStage)))