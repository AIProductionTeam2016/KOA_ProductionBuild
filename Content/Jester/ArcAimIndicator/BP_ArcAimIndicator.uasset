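; BP_ArcAimIndicator draws a ballistic aim arc from a start to a target position, rebuilt every tick while enabled.
; It solves a launch velocity in the Y-Z plane, exposed through GetTargetStartVelocity, then simulates gravity in sub-stepped segments.
; Line traces end the arc at the first hit.
; The resulting spline points are rendered with spline mesh components, destroyed and recreated each update.
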(event EventBeginPlay)

(event Collision|EventActorBeginOverlap
  (params (OtherActor :type Actor%20Object%20Reference)))

(event EventTick
  (params (DeltaSeconds :type Float%20%28single-precision%29))
  (if (Variables|Default|GetEnabled)
    (CallFunction|CreateSplinePoints)
    (CallFunction|DeleteSplineMeshes)
    (CallFunction|CreateSplineMesh)))

(fn ConstructionScript)

(fn CreateSplineMesh
  (bind _spline (Variables|Default|GetSpline))
  (CallFunction|DeleteSplineMeshes)
  (for _index (range 1 (- (Spline|GetNumberOfSplinePoints _spline) 1))
    (bind _returnvalue (AddComponent|AddSplineMeshComponent false))
    (Utilities|Array|Add (Variables|Default|GetSplineMeshComponents) _returnvalue)
    (SplineMesh|SetStartandEnd _returnvalue (Spline|GetLocationatSplinePoint _spline (- _index 1) "Local") (Spline|GetTangentatSplinePoint _spline (- _index 1) "Local") (Spline|GetLocationatSplinePoint _spline _index "Local") (Spline|GetTangentatSplinePoint _spline _index "Local") true :!class /Script/Engine.SplineMeshComponent)
    (SplineMesh|SetStartScale _returnvalue "(X=0.200000,Y=0.200000)" true :!class /Script/Engine.SplineMeshComponent)
    (SplineMesh|SetEndScale _returnvalue "(X=0.200000,Y=0.200000)" true :!class /Script/Engine.SplineMeshComponent)))

(fn CreateSplinePoints
  (bind _targetposition (Variables|Default|GetTargetPosition))
  (bind _segtimestep (Variables|Default|GetsegTimeStep))
  (bind _startposition (Variables|Default|GetStartPosition))
  (bind _segtimenumsubsteps (Variables|Default|GetsegTimeNumSubSteps))
  (bind _returnvalue (Math|Conversions|ToFloat(Integer) _segtimenumsubsteps))
  (bind _returnvalue_2 (- _targetposition _startposition))
  (bind (_x _y _z) (Math|Vector|BreakVector _returnvalue_2))
  (bind _returnvalue_3 (/ _segtimestep _returnvalue))
  (LocalVariables|SetdiffX _y)
  (LocalVariables|SetdiffY _z)
  (LocalVariables|SetstartVelX (|(((sqrt(g))*x)/((sqrt(2))*(pow(((x*x)+(y*y)),(1/4.000000))))) (Variables|Default|GetGravity) (LocalVariables|GetdiffX) (LocalVariables|GetdiffY)))
  (LocalVariables|SetstartVelY (|(((g*x)/(2*vx))+((vx*y)/x)) (Variables|Default|GetGravity) (LocalVariables|GetdiffX) (LocalVariables|GetstartVelX) (LocalVariables|GetdiffY)))
  (LocalVariables|Setvelocity (Math|Vector|MakeVector 0.0 (LocalVariables|GetstartVelX) (LocalVariables|GetstartVelY)))
  (Variables|Default|SetTargetStartVelocity (Math|Vector|MakeVector 0.0 (LocalVariables|GetstartVelX) (LocalVariables|GetstartVelY)))
  (LocalVariables|Setposition (Variables|Default|GetStartPosition))
  (Spline|ClearSplinePoints (Variables|Default|GetSpline))
  (Utilities|FlowControl|ForLoopwithBreak 1 (Variables|Default|GetmaxSegments) :!label _label
    (:LoopBody
      (Spline|AddSplinePoint (Variables|Default|GetSpline) (LocalVariables|Getposition) "World")
      (LocalVariables|SetnewPosition (LocalVariables|Getposition))
      (for _index (range 1 (Variables|Default|GetsegTimeNumSubSteps))
        (LocalVariables|SetnewPosition (+ (LocalVariables|GetnewPosition) (* (LocalVariables|Getvelocity) _returnvalue_3)))
        (LocalVariables|Setvelocity (+ (LocalVariables|Getvelocity) (Math|Vector|MakeVector 0.0 0.0 (* (Variables|Default|GetGravity) _returnvalue_3 -1.0)))))
      (bind (_outhit _returnvalue_4) (Collision|LineTraceForObjects (LocalVariables|Getposition) (LocalVariables|GetnewPosition) (Variables|Default|GetCollisionObjectTypes) false 0 "None"))
      (if _returnvalue_4
        (LocalVariables|Setposition (.Location (Collision|BreakHitResult _outhit)))
        (goto _label Break)
        (else
          (LocalVariables|Setposition (LocalVariables|GetnewPosition)))))
    (:Completed
      (Spline|AddSplinePoint (Variables|Default|GetSpline) (LocalVariables|Getposition) "World"))))

(fn DeleteSplineMeshes
  (for _array_element (Variables|Default|GetSplineMeshComponents)
    (Components|DestroyComponent _array_element))
  (Utilities|Array|Clear (Variables|Default|GetSplineMeshComponents)))

(fn GetTargetStartVelocity
  (return (Variables|Default|GetTargetStartVelocity)))