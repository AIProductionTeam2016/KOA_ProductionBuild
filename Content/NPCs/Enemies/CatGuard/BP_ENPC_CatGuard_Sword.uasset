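; Sword-wielding Cat Guard enemy NPC that adds health bar hookup and a bleeding effect.
; On BeginPlay it passes itself as the enemy reference to its EnemyHealthBar widget.
; Tick polls IsBleeding every frame to show or hide the bleeding particle component.
; A check that disables capsule collision on death is present but unconnected, so it never runs.
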(event `self.ReceiveBeginPlay`
  ;[1 1 1] Set REF_EnemyHPBar
  (bind _aswbp_ui_enemy_health_bar (cast `/Game/UI/NPC/WBP_UI_EnemyHealthBar` (`WidgetComponent.GetUserWidgetObject` (`self.EnemyHealthBar`))))
  (set `/Game/UI/NPC/WBP_UI_EnemyHealthBar.REF_BASE_Enemy` self _aswbp_ui_enemy_health_bar))

(event `self.ReceiveActorBeginOverlap`
  (params (OtherActor :type "Actor Object Reference")))

(event `self.ReceiveTick`
  (params (DeltaSeconds :type "Float (single-precision)"))
  (bind _ps_ss_bleeding (`self.PS_SS_BLEEDING`))
  ;[1 1 1] IS BLEEDING
  (if (`self.IsBleeding`)
    (`SceneComponent.SetVisibility` _ps_ss_bleeding true true)
    (else
      (`SceneComponent.SetVisibility` _ps_ss_bleeding false false))))

(fn `UserConstructionScript`)