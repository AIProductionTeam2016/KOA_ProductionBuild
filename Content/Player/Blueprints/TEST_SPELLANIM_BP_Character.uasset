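; Test player character Blueprint that sets up the in-game HUD and swaps the mouse cursor on input.
; BeginPlay creates UI_InGameHUD, stores a reference, adds it to the viewport and sets game-only input mode.
; Holding E shows a crosshair cursor, and releasing it restores the default.
; Tick calls UpdateCursor, which is empty; disconnected nodes hold unfinished mouse-to-world and screen-offset experiments.
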(event `/Game/Player/Blueprints/BP_KOA_PROTO_Character.ReceiveBeginPlay`
  ;[1 1 1] BeginPlay: Create HUD, Save a reference, Add it to viewport, set input mode
  (bind _returnvalue (`|CreateWidget` "/Game/Game/UI/UI/UI_InGameHUD.UI_InGameHUD_C"))
  (bind _output_get (set `self.REF_InGameHUD` _returnvalue))
  (`UserWidget.AddToViewport` _output_get 0)
  (`WidgetBlueprintLibrary.SetInputMode_GameOnly` null))

(event `Key|E`
  (params (Key :type "Key Structure" :default "AnyKey"))
  (bind _returnvalue (`GameplayStatics.GetPlayerController` 0))
  (:`Pressed`
    (set `PlayerController.CurrentMouseCursor` "Crosshairs" _returnvalue))
  (:`Released`
    (set `PlayerController.CurrentMouseCursor` "Default" _returnvalue)))

(event `/Game/Player/Blueprints/BP_KOA_PROTO_Character.ReceiveTick`
  (params (DeltaSeconds :type "Float (single-precision)"))
  ;[1 1 1] Event Tick: Move Cursor
  (`self.UpdateCursor`))

(fn `UpdateCursor`)

(fn `UserConstructionScript`)