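; Vampire dual daggers artifact with two hold-and-release abilities: blink-style backstab aiming (E) and Blood Storm (R).
; E switches camera mode, turns an aiming mesh by the nearest sphere-traced enemy's side, then rotates the player capsule on release; the backstab branch is empty.
; R grows a sphere collecting overlapped enemies, then fires tendril projectiles at them on release.
; Damage events hurt them and send helix tendrils back; heal events heal per enemy.
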(event EventOnPressAbilityE
  (bind _camera (Variables|Default|GetCamera))
  (CallFunction|AimingMeshInit)
  (bind _succeeded (CallFunction|GetCamera))
  (if _succeeded
    (Variables|/Game/Game/Camera/BP_ControlledCamera.BP_ControlledCamera_C|SetcameraMode _camera "NewEnumerator2")
    (Variables|/Game/Game/Camera/BP_ControlledCamera.BP_ControlledCamera_C|SetCA_MaxAimDistance _camera 8e+02)))

(event EventOnBloodStormDamage
  (CallFunction|BloodStormHurtEnemies)
  (CallFunction|BloodStormRecieveProj))

(event EventOnBloodStormHeal
  (CallFunction|BloodStormHealPlayer))

(event EventOnPressAbilityR
  (CallFunction|BloodStormInit))

(event EventOnReleaseAbilityR
  (CallFunction|BloodStormEnd))

(event EventOnReleaseAbilityE
  (CallFunction|AimingMeshEnd)
  (bind _succeeded (CallFunction|GetCamera))
  (if _succeeded
    (Variables|/Game/Game/Camera/BP_ControlledCamera.BP_ControlledCamera_C|SetcameraMode (Variables|Default|GetCamera) "NewEnumerator0")))

(event EventOnTick
  (params (deltaTime :type Float%20%28single-precision%29))
  (CallFunction|AimingMeshTick deltaTime)
  (CallFunction|BloodStormTick deltaTime))

(fn GetCamera
  (Utilities|IsValid (Variables|Default|GetCamera)
    (:Is%20Valid
      (return (Variables|Default|GetCamera) true))
    (:Is%20Not%20Valid
      (bind _asbp_controlled_camera (Utilities|Casting|CastToBP_ControlledCamera (Pawn|GetViewTarget (Game|GetPlayerController (Class|KOAArtifactDualDaggers|GetPlayer))))
        (:then
          (bind _output_get (Variables|Default|SetCamera _asbp_controlled_camera))
          (return _output_get true))
        (:CastFailed
          (return (Variables|Default|GetCamera) false))))))

(fn AimingMeshInit
  (bind _returnvalue (Class|KOAArtifactDualDaggers|GetPlayer))
  (bind _vd_e_aimingmeshcomponent (Variables|/Script/KOA_PROTO.KOA_PROTO_Character|GetVD_E_AimingMeshComponent _returnvalue))
  (Components|SkeletalMesh|SetAnimInstanceClass (Variables|/Script/KOA_PROTO.KOA_PROTO_Character|GetVD_E_AimingMeshComponent (Class|KOAArtifactDualDaggers|GetPlayer)) "/Game/Artifacts/VampireDaggers/Abilities/AnimationBlueprints/AnimBP_DualDaggerBlink.AnimBP_DualDaggerBlink_C")
  (Variables|Blink|SetE_ShouldTick true)
  (bind _asanim_bp_dual_dagger_blink (Utilities|Casting|CastToAnimBP_DualDaggerBlink (Components|SkeletalMesh|GetAnimInstance _vd_e_aimingmeshcomponent)))
  (Variables|Blink|SetanimBP_Blink _asanim_bp_dual_dagger_blink)
  (Variables|Default|SetaimingMesh_Blink _vd_e_aimingmeshcomponent))

(fn AimingMeshTick
  (params (DeltaTime :type Float%20%28single-precision%29))
  (bind _aimingmesh_blink (Variables|Default|GetaimingMesh_Blink))
  (bind _aimingmesh_blink_2 (Variables|Default|GetaimingMesh_Blink))
  (bind _e_enemydistance (Variables|Blink|GetE_enemyDistance))
  (bind _returnvalue (Transformation|GetWorldLocation _aimingmesh_blink_2))
  (bind _returnvalue_2 (Math|Vector|MakeVector 0.0 _e_enemydistance 0.0))
  (bind _returnvalue_3 (Transformation|GetWorldRotation _aimingmesh_blink))
  (bind _returnvalue_4 (+ _returnvalue "0, 0,75.000000"))
  (if (Variables|Blink|GetE_ShouldTick)
    (LocalVariables|Set_DeltaTime DeltaTime)
    (Variables|Blink|SetE_shouldBackStab false)
    (Variables|/Game/Artifacts/VampireDaggers/Abilities/AnimationBlueprints/AnimBP_DualDaggerBlink.AnimBP_DualDaggerBlink_C|SetcanBackStab (Variables|Blink|GetanimBP_Blink) false)
    (bind _outhits (Collision|MultiSphereTraceForObjects (Class|KOAArtifactDualDaggers|GetPlayer) (+ _returnvalue_4 _returnvalue_2) (- _returnvalue_4 _returnvalue_2) 1e+01 (Utilities|Array|MakeArray "ObjectTypeQuery3") false 0 "None"))
    (bind _array_element (Utilities|Array|ForEachLoopwithBreak _outhits)
      (:LoopBody
        (Utilities|Casting|CastToKOA_BASE_EnemyCharacter (.HitActor (Collision|BreakHitResult _array_element)))
        (Variables|/Game/Artifacts/VampireDaggers/Abilities/AnimationBlueprints/AnimBP_DualDaggerBlink.AnimBP_DualDaggerBlink_C|SetcanBackStab (Variables|Blink|GetanimBP_Blink) true)
        (Variables|Blink|SetE_shouldBackStab true)
        (Utilities|Array|Add (LocalVariables|GettracedActorLocations) (Transformation|GetActorLocation (.HitActor (Collision|BreakHitResult _array_element)))))
      (:Completed
        (if (Variables|Blink|GetE_shouldBackStab)
          (LocalVariables|SetclosestActorDistance 1e+04)
          (for _array_element_2 (LocalVariables|GettracedActorLocations)
            (if (<= (Math|Vector|VectorLength (- _array_element_2 (Transformation|GetWorldLocation (Variables|Default|GetaimingMesh_Blink)))) (LocalVariables|GetclosestActorDistance))
              (LocalVariables|SetclosestActorDistance (Math|Vector|VectorLength (- _array_element_2 (Transformation|GetWorldLocation (Variables|Default|GetaimingMesh_Blink)))))
              (LocalVariables|SetclosestActorLocation _array_element_2)))
          (Math|Float|CompareFloat (.Y (Math|Vector|BreakVector (- (LocalVariables|GetclosestActorLocation) (Transformation|GetWorldLocation _aimingmesh_blink)))) 0.0
            (:>
              (Transformation|SetWorldRotation _aimingmesh_blink (Class|KismetMathLibrary|RInterptoConstant _returnvalue_3 "0, 0, 0" (LocalVariables|Get_DeltaTime) (Variables|Blink|GetE_meshTurnSpeed)) false false))
            (:==
              (Transformation|SetWorldRotation _aimingmesh_blink (Class|KismetMathLibrary|RInterptoConstant _returnvalue_3 "0,180.000000, 0" (LocalVariables|Get_DeltaTime) (Variables|Blink|GetE_meshTurnSpeed)) false false :!label _label))
            (:<
              (goto _label))))))))

(fn AimingMeshEnd
  (Variables|Blink|SetE_ShouldTick false)
  (Transformation|SetWorldRotation (Variables|/Script/Engine.Character|GetCapsuleComponent (Class|KOAArtifactDualDaggers|GetPlayer)) (Math|Rotator|CombineRotators (Transformation|GetWorldRotation (Variables|Default|GetaimingMesh_Blink)) "0,90.000000, 0") false false)
  (if (Variables|Blink|GetE_shouldBackStab)
    _))

(fn BloodStormInit
  (Transformation|SetActorTransform (Variables|Default|GetBloodStormSphere) (Math|Transform|MakeTransform (+ (Transformation|GetActorLocation (Class|KOAArtifactDualDaggers|GetPlayer)) (Math|Vector|MakeVector 0.0 0.0 (Variables|BloodStorm|GetR_sphereZOffset))) "0, 0, 0" "0.000000,0.000000,0.000000") false true)
  (Variables|BloodStorm|SetR_shouldTick true)
  (Variables|BloodStorm|SetR_sphereSize 0.0)
  (Utilities|Array|Clear (Variables|BloodStorm|GetR_TrackedEnemies)))

(fn BloodStormTick
  (params (deltaTime :type Float%20%28single-precision%29))
  (bind _bloodstormsphere (Variables|Default|GetBloodStormSphere))
  (bind _returnvalue (Transformation|GetActorTransform _bloodstormsphere))
  (bind (_location _rotation) (Math|Transform|BreakTransform _returnvalue))
  (if (Variables|BloodStorm|GetR_shouldTick)
    (Variables|BloodStorm|SetR_sphereSize (Math|Float|Clamp(Float) (+ (Variables|BloodStorm|GetR_sphereSize) (* (Variables|BloodStorm|GetR_sphereGrowSpeed) deltaTime)) 0.0 (/ (.MaxCastRange (Utilities|Struct|BreakAbilityStats (Class|KOABASEArtifact|GetAbilityStats "ABID_R"))) (Variables|BloodStorm|GetR_sphereMeshRadius))))
    (Transformation|SetActorTransform _bloodstormsphere (Math|Transform|MakeTransform _location _rotation (Math|Conversions|ToVector(Float) (Variables|BloodStorm|GetR_sphereSize))) false true)
    (bind _asbp_blood_storm_sphere (Utilities|Casting|CastToBP_BloodStormSphere (Variables|Default|GetBloodStormSphere)))
    (for _array_element (Collision|GetOverlappingActors (Variables|/Game/Artifacts/VampireDaggers/BP_BloodStormSphere.BP_BloodStormSphere_C|GetHemisphereMesh _asbp_blood_storm_sphere) "/Script/KOA_PROTO.KOA_BASE_EnemyCharacter" :!class /Script/Engine.PrimitiveComponent)
      (bind _askoa_base_enemy_character (Utilities|Casting|CastToKOA_BASE_EnemyCharacter _array_element))
      (Utilities|Array|AddUnique (Variables|BloodStorm|GetR_TrackedEnemies) _askoa_base_enemy_character))))

(fn BloodStormEnd
  (Variables|BloodStorm|SetR_shouldTick false)
  (CallFunction|BloodStormSendProj))

(fn BloodStormSendProj
  (bind _abilr_squigglytendrillifetime (Variables|Default|GetABILR_SquigglyTendrilLifeTime))
  (for _array_element (Variables|BloodStorm|GetR_TrackedEnemies)
    (bind _returnvalue (Class|KOAArtifactDualDaggers|SpawnSquigglyProjectile (Transformation|GetActorLocation (Class|KOAArtifactDualDaggers|GetPlayer))))
    (bind _asbp_vdbs_squiggly_projectile (Utilities|Casting|CastToBP_VDBS_SquigglyProjectile _returnvalue))
    (Variables|/Script/KOA_PROTO.BASE_Projectile|SetTargetLocation _asbp_vdbs_squiggly_projectile (Transformation|GetActorLocation _array_element))
    (Variables|/Script/KOA_PROTO.AMTA_Projectile_Squiggly|SetProjLifeTime _asbp_vdbs_squiggly_projectile _abilr_squigglytendrillifetime)
    (Variables|/Script/KOA_PROTO.AMTA_Projectile_Squiggly|SetProjTimeBeforeDelete _asbp_vdbs_squiggly_projectile (+ _abilr_squigglytendrillifetime 1.0))
    (Variables|/Game/Artifacts/VampireDaggers/BP_VDBS_SquigglyProjectile.BP_VDBS_SquigglyProjectile_C|SetTargetActor _asbp_vdbs_squiggly_projectile _array_element)))

(fn BloodStormRecieveProj
  (bind _returnvalue (Class|KOAArtifactDualDaggers|GetPlayer))
  (bind _abilr_helixtendrillifetime (Variables|Default|GetABILR_HelixTendrilLifeTime))
  (for _array_element (Variables|BloodStorm|GetR_TrackedEnemies)
    (for _index (range 1 (Variables|BloodStorm|GetR_TendrilsPerEnemy))
      (bind _returnvalue_2 (Class|KOAArtifactDualDaggers|SpawnHelixProjectile (Transformation|GetActorLocation _array_element)))
      (bind _asbp_vdbs_helix_seek_projectile (Utilities|Casting|CastToBP_VDBS_HelixSeekProjectile _returnvalue_2))
      (Variables|/Script/KOA_PROTO.AMTA_Projectile_HelixSeek|SetProjLifeTime _asbp_vdbs_helix_seek_projectile _abilr_helixtendrillifetime)
      (Variables|/Script/KOA_PROTO.AMTA_Projectile_HelixSeek|SetProjTimeBeforeDelete _asbp_vdbs_helix_seek_projectile (+ _abilr_helixtendrillifetime 1.0))
      (Variables|/Script/KOA_PROTO.BASE_Projectile|SetTargetLocation _asbp_vdbs_helix_seek_projectile (Transformation|GetActorLocation _returnvalue))
      (Variables|/Game/Artifacts/VampireDaggers/BP_VDBS_HelixSeekProjectile.BP_VDBS_HelixSeekProjectile_C|SetTargetActor _asbp_vdbs_helix_seek_projectile _returnvalue))))

(fn BloodStormHealPlayer
  (for _array_element (Variables|BloodStorm|GetR_TrackedEnemies)
    (Class|KOAPROTOCharacter|HealPlayer (Class|KOAArtifactDualDaggers|GetPlayer) (Variables|Default|GetABILR_HealAmount)))
  (Utilities|Array|Clear (Variables|BloodStorm|GetR_TrackedEnemies)))

(fn BloodStormHurtEnemies
  (for _array_element (Variables|BloodStorm|GetR_TrackedEnemies)
    (Class|KOABASEEnemyCharacter|ReceiveDamage _array_element (.HitDamage (Utilities|Struct|BreakAbilityStats (Class|KOABASEArtifact|GetAbilityStats "ABID_R"))))))