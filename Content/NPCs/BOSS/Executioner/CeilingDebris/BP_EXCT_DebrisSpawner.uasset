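; Ceiling debris spawner for the Executioner boss that drops debris around the player and adds a Cat Guard enemy.
; Every tick it teleports to match the Jester's Y position, keeping its own X and Z.
; StartDebrisDrop runs a looping timer that spawns debris at random Y offsets within Range until the set count is reached.
; The same call immediately spawns one random-type Cat Guard with its default controller at the spawner.
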(event EventBeginPlay
  (bind _aspcbp_jester (Utilities|Casting|CastToPCBP_Jester (Game|GetPlayerCharacter 0)))
  (Variables|Default|SetREF_Jester _aspcbp_jester))

(event EventActorBeginOverlap
  (params (OtherActor :type Actor%20Object%20Reference)))

(event EventTick
  (params (DeltaSeconds :type Float%20%28single-precision%29))
  (CallFunction|SetYLocation))

(fn ConstructionScript)

(fn SetYLocation
  (bind _defaultsceneroot (Variables|Default|GetDefaultSceneRoot))
  (bind _returnvalue (Transformation|GetWorldLocation _defaultsceneroot))
  (bind (_x _y _z) (Math|Vector|BreakVector _returnvalue))
  (Transformation|SetActorLocation (Math|Vector|MakeVector _x (.Y (Math|Vector|BreakVector (Transformation|GetActorLocation (Variables|Default|GetREF_Jester)))) _z) false true))

(fn CreateDebris
  (bind _range (Variables|Default|Getrange))
  (if (< (Variables|Default|GetnumDebrisDropped) (Variables|Default|GetnumDebrisToDrop))
    (Game|SpawnActorfromClass "/Game/NPCs/BOSS/Executioner/CeilingDebris/BP_EXCT_CeilingDebris.BP_EXCT_CeilingDebris_C" (Math|Transform|MakeTransform (+ (Transformation|GetActorLocation) (Math|Vector|MakeVector 0.0 (Math|Random|RandomFloatinRange (* _range -1.0) _range) 0.0))) "AdjustIfPossibleButAlwaysSpawn" self 0)
    (Math|Integer|IncrementInt (Variables|Default|GetnumDebrisDropped))
    (else
      (Class|KismetSystemLibrary|ClearTimerHandle (Variables|Default|GetHND_DebrisTimer)))))

(fn StartDebrisDrop
  (bind _returnvalue (Utilities|Time|SetTimerbyFunctionName 0 "CreateDebris" (Variables|Default|GettimeBetweenDebris) true))
  (Variables|Default|SetHND_DebrisTimer _returnvalue)
  (Variables|Default|SetnumDebrisDropped 0)
  (CallFunction|CreateEnemy))

(fn CreateEnemy
  (LocalVariables|SetTOFCatGuard (Math|Random|RandomInteger (|GetNumEnumEntries)))
  (bind _returnvalue (Game|SpawnActorfromClass "/Game/NPCs/Enemies/CatGuard/BP_ENPC_CatGuard.BP_ENPC_CatGuard_C" (Transformation|GetWorldTransform (Variables|Default|GetDefaultSceneRoot)) "Undefined" 0 0 (Utilities|Enum|ByteToEnumETYPEOF_CatGuard (Math|Conversions|ToByte(Integer) (LocalVariables|GetTOFCatGuard)))))
  (Pawn|SpawnDefaultController _returnvalue))