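; Character Blueprint for the Cat Guard enemy NPC, with an overhead or attached health bar widget component.
; On BeginPlay it casts that widget to WBP_UI_EnemyHealthBar and passes itself in as the enemy reference.
; Every Tick it polls GetIsDead and, while dead, sets the capsule's collision to NoCollision.
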(event `self.ReceiveBeginPlay`
  ;[1 1 1] Set REF_EnemyHPBar
  (bind _aswbp_ui_enemy_health_bar (cast `/Game/UI/NPC/WBP_UI_EnemyHealthBar` (`WidgetComponent.GetUserWidgetObject` (`self.EnemyHealthBar`))))
  (set `/Game/UI/NPC/WBP_UI_EnemyHealthBar.REF_BASE_Enemy` self _aswbp_ui_enemy_health_bar))

(event `self.ReceiveActorBeginOverlap`
  (params (OtherActor :type "Actor Object Reference")))

(event `self.ReceiveTick`
  (params (DeltaSeconds :type "Float (single-precision)"))
  (if (`self.GetIsDead` self)
    (`PrimitiveComponent.SetCollisionEnabled` (`self.CapsuleComponent`) "NoCollision")))

(fn `UserConstructionScript`)